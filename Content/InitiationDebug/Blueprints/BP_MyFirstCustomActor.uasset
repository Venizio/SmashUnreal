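; BP_MyFirstCustomActor is a debug actor that exercises variable access and function calls, printing the results on BeginPlay.
; It sets MyBlueprintReadWriteFloat to ten and prints it through two local helper functions.
; It then calls PrintMyBodyIsReadyOnScreen and prints the result of GetTenValue, both defined outside this graph, likely in a native parent class.
; Tick, overlap and construction logic are empty.
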(event `self.ReceiveBeginPlay`
  (`self.WriteTenOnReadWriteFloat`)
  (`self.PrintReadWriteFloat`)
  (`self.PrintMyBodyIsReadyOnScreen`)
  (`KismetSystemLibrary.PrintString` (`KismetStringLibrary.Conv_IntToString` (`self.GetTenValue`))))

(fn `PrintReadWriteFloat`
  (`KismetSystemLibrary.PrintString` (`KismetStringLibrary.Conv_DoubleToString` (`self.MyBlueprintReadWriteFloat`))))

(fn `UserConstructionScript`)

(fn `WriteTenOnReadWriteFloat`
  (set `self.MyBlueprintReadWriteFloat` 10.0))